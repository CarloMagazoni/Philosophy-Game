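; Foma (Thomas Aquinas) NPC Blueprint that opens staged dialogue when the player presses Interact nearby.
; A box overlap toggles proximity and input; interacting disables player character input, shows the cursor and opens the widget matching the speech counter.
; The first and two fail dialogues also set test or fail flags on the Zasovs, book and fountain actors.
; The changespeech event sets the counter, or increments it when passed -1.
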(event OnComponentBeginOverlap(Box)
  (params (OverlappedComponent :type Primitive%20Component%20Object%20Reference) (OtherActor :type Actor%20Object%20Reference) (OtherComp :type Primitive%20Component%20Object%20Reference) (OtherBodyIndex :type Integer) (bFromSweep :type Boolean) (SweepResult :type Hit%20Result%20Structure%20%28by%20ref%29))
  ;[0.3504 0.8287 1] is Player Near
  (Variables|Default|SetplayerNear true)
  (Input|EnableInput (Game|GetPlayerController 0)))

(event OnComponentEndOverlap(Box)
  (params (OverlappedComponent :type Primitive%20Component%20Object%20Reference) (OtherActor :type Actor%20Object%20Reference) (OtherComp :type Primitive%20Component%20Object%20Reference) (OtherBodyIndex :type Integer))
  ;[0.3504 0.8287 1] is Player Near
  (Variables|Default|SetplayerNear false)
  (Input|DisableInput (Game|GetPlayerController 0)))

(event Custom|change%20speech
  (params (new%20count :type Integer))
  ;[1 0.2222 0] set number of speech
  (if (== new%20count -1)
    (bind _result (Math|Integer|IncrementInt (Variables|Default|GetcountSpeech))
      (:%20%20
        (if (== _result 3)
          _)))
    (else
      (Variables|Default|SetcountSpeech new%20count))))

(event Input|ActionEvents|InputActionInteract
  (params (Key :type Key%20Structure :default "None"))
  (bind _returnvalue (Game|GetPlayerController 0))
  ;[1 0.985 0.1271] setting Dialog
  (:Pressed
    (if (Variables|Default|GetplayerNear)
      (Input|DisableInput (Game|GetPlayerCharacter 0) _returnvalue)
      (switch int (Variables|Default|GetcountSpeech)
        (:0
          (bind _returnvalue_2 (UserInterface|CreateWidget "/Game/Quests/quest_5_gate/FA/fa_first_dialog.fa_first_dialog_C"))
          (UserInterface|Viewport|AddtoViewport _returnvalue_2 0)
          (bind _returnvalue_3 (Actor|GetActorOfClass "/Game/Quests/quest_5_gate/zasovs.zasovs_C"))
          (Variables|/Game/Quests/quest_5_gate/zasovs.zasovs_C|SetisTestValible _returnvalue_3 true))
        (:1
          (bind _returnvalue_4 (UserInterface|CreateWidget "/Game/Quests/quest_5_gate/FA/fa_fail_dialog_1.fa_fail_dialog_1_C"))
          (UserInterface|Viewport|AddtoViewport _returnvalue_4 0)
          (bind _returnvalue_5 (Actor|GetActorOfClass "/Game/Quests/quest_5_gate/tableBook/book_.book__C"))
          (Variables|/Game/Quests/quest_5_gate/tableBook/book_.book__C|SetisFail _returnvalue_5 true))
        (:2
          (bind _returnvalue_6 (UserInterface|CreateWidget "/Game/Quests/quest_5_gate/FA/fa_fail_dialog_2.fa_fail_dialog_2_C"))
          (UserInterface|Viewport|AddtoViewport _returnvalue_6 0)
          (bind _returnvalue_7 (Actor|GetActorOfClass "/Game/Arcitecture/Architecture/Fountan_Big_BP.Fountan_Big_BP_C"))
          (Variables|/Game/Arcitecture/Architecture/Fountan_Big_BP.Fountan_Big_BP_C|SetisFail _returnvalue_7 true))
        (:3
          (bind _returnvalue_8 (UserInterface|CreateWidget "/Game/Quests/quest_5_gate/FA/fa_ending_dialog.fa_ending_dialog_C"))
          (UserInterface|Viewport|AddtoViewport _returnvalue_8 0)))
      (Variables|/Script/Engine.PlayerController|SetbShowMouseCursor _returnvalue true))))

(fn ConstructionScript)