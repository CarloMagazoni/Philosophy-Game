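; A one-shot cutscene camera actor that takes over player 0's view and disables character input when CameraSwitch is called.
; In spline mode, a timeline with adjustable play rate drives the camera's location and rotation along the spline of a referenced SplineBP.
; After a delay, started from the timeline's update in spline mode or directly otherwise, it returns view and input to the character and destroys itself.
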(event EventCameraSwitch
  (if (Variables|Default|GetIsASplineCamera)
    (Variables|Default|SetSpline (Variables|/Game/Camera/SplineBP.SplineBP_C|GetSpline (Variables|Default|GetSplineBP))))
  (Game|Player|SetViewTargetwithBlend (Game|GetPlayerController 0) self 0.0 "VTBlend_Linear" 0.0 false)
  (Input|DisableInput (Game|GetPlayerCharacter 0) (Game|GetPlayerController 0))
  (if (Variables|Default|GetIsASplineCamera)
    (Components|Timeline|SetPlayRate (Variables|Default|GetTimeline_0) (Variables|Default|GetPlayrate%28Timeline%20Speed%29))
    (bind _animationalpha (Timeline|Timeline_0 Play)
      (:Update
        (Transformation|SetWorldTransform (Variables|Default|GetCamera) (Math|Transform|MakeTransform (Spline|GetLocationatDistanceAlongSpline (Variables|Default|GetSpline) (* _animationalpha (Spline|GetSplineLength (Variables|Default|GetSpline))) "World") (Spline|GetRotationatDistanceAlongSpline (Variables|Default|GetSpline) (* _animationalpha (Spline|GetSplineLength (Variables|Default|GetSpline))) "World")) false false)
        (Utilities|FlowControl|Delay (Variables|Default|GetTimeline%20Length%20+%20Delay))))
    (else
      (Utilities|FlowControl|Delay (Variables|Default|GetDelay%20W/O%20Spline))))
  (Game|Player|SetViewTargetwithBlend (Game|GetPlayerController 0) (Game|GetPlayerCharacter 0) 0.0 "VTBlend_Linear" 0.0 false)
  (Input|EnableInput (Game|GetPlayerCharacter 0) (Game|GetPlayerController 0))
  (Actor|DestroyActor))

(fn ConstructionScript)