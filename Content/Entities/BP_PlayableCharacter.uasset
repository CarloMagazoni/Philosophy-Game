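; Player character with health, toggleable melee combat, physics object carrying and first-/third-person camera switching.
; Attacks drive CharacterAnimBP flags and apply damage through three delayed forward box traces, with persistent debug drawing.
; A camera line trace grabs objects via PhysicsHandle, following a wheel-adjustable GrabLocation on Tick, which first-person mode enables and third-person disables.
; Damage updates the StatsWidget health bar; death shows GameOverWidget and destroys the actor.
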(event Custom|Pick%20Up
  (bind _followcamera (Variables|Default|GetFollowCamera))
  (bind _returnvalue (Transformation|GetWorldLocation _followcamera))
  ;[1 1 1] Pick Up - Drop
  (bind (_outhit _returnvalue_2) (Collision|LineTraceByChannel _returnvalue (+ _returnvalue (* (Math|Vector|GetForwardVector _followcamera) 2.5e+02)) "TraceTypeQuery3" false 0 "None"))
  (if _returnvalue_2
    (Variables|Default|SetPhysics%20Object (.HitComponent (Collision|BreakHitResult _outhit)))
    (Class|PhysicsHandleComponent|GrabComponentatLocation (Variables|Default|GetPhysicsHandle) (.HitComponent (Collision|BreakHitResult _outhit)) "None" (Physics|GetCenterOfMass (.HitComponent (Collision|BreakHitResult _outhit)) "None"))
    (Variables|Default|SetisHoldingObject true)
    (Class|EvilInformaionInterface|Info(Message) (.HitActor (Collision|BreakHitResult _outhit)))
    (Class|PrimitiveComponent|SetAngularDamping (Variables|Default|GetPhysics%20Object) 0.0)
    (Variables|/Script/Engine.CharacterMovementComponent|SetMaxWalkSpeed (Variables|Character|GetCharacterMovement) 3e+02)))

(event Custom|Drop
  (bind _grablocation (Variables|Default|GetGrabLocation))
  (bind _physics_object (Variables|Default|GetPhysics%20Object))
  (bind _relativelocation (Variables|/Script/Engine.SceneComponent|GetRelativeLocation _grablocation))
  ;[1 1 1] Pick Up - Drop
  (Physics|Components|PhysicsHandle|ReleaseComponent (Variables|Default|GetPhysicsHandle))
  (Variables|Default|SetisHoldingObject false)
  (Class|PrimitiveComponent|SetAllPhysicsLinearVelocity _physics_object "0, 0, 0" false)
  (Utilities|FlowControl|Delay 0.2)
  (Class|PrimitiveComponent|SetAngularDamping _physics_object 1e+01)
  (Variables|/Script/Engine.CharacterMovementComponent|SetMaxWalkSpeed (Variables|Character|GetCharacterMovement) 5e+02)
  (Transformation|SetRelativeLocation _grablocation (Math|Vector|MakeVector 3e+02 (.y _relativelocation) (.z _relativelocation)) false true))

(event EventTick
  (params (DeltaSeconds :type Float%20%28single-precision%29))
  ;[1 1 1] Pick Up - Drop
  (Physics|Components|PhysicsHandle|SetTargetLocation (Variables|Default|GetPhysicsHandle) (Transformation|GetWorldLocation (Variables|Default|GetGrabLocation))))

(event EventSwitchCameraModeFps
  ;[1 1 1] Pick Up - Drop
  (Actor|Tick|SetActorTickEnabled true)
  (Components|Activation|Deactivate (Variables|Default|GetCameraComponent))
  (Components|Activation|Activate (Variables|Default|GetFollowCamera) false)
  (Class|PrimitiveComponent|SetOwnerNoSee (Variables|Character|GetMesh) true)
  (Variables|/Script/Engine.CharacterMovementComponent|SetMaxWalkSpeed (Variables|Character|GetCharacterMovement) 3e+02))

(event EventBeginPlay
  ;[1 1 1] Damage/CombatMode/Stats
  (bind _returnvalue (UserInterface|CreateWidget "/Game/Elf/Stats/StatsWidget.StatsWidget_C"))
  (UserInterface|Viewport|AddtoViewport _returnvalue 0)
  (bind _ascharacter_anim_bp (Utilities|Casting|CastToCharacterAnimBP (Components|SkeletalMesh|GetAnimInstance (Variables|Character|GetMesh))))
  (Variables|Default|SetAnimationBP _ascharacter_anim_bp))

(event Game|Damage|EventAnyDamage
  (params (Damage :type Float%20%28single-precision%29) (DamageType :type Damage%20Type%20Object%20Reference) (InstigatedBy :type Controller%20Object%20Reference) (DamageCauser :type Actor%20Object%20Reference))
  ;[1 1 1] Damage/CombatMode/Stats
  (CallFunction|TakeDamageFunction Damage)
  (if (<= (Variables|Default|GetHealth) 0.0)
    (Viewport|RemoveAllWidgets)
    (bind _returnvalue (UserInterface|CreateWidget "/Game/Elf/Stats/GameOverWidget.GameOverWidget_C"))
    (UserInterface|Viewport|AddtoViewport _returnvalue 0)
    (Actor|DestroyActor)
    (Variables|/Script/Engine.PlayerController|SetbShowMouseCursor (Game|GetPlayerController 0) true)))

(event EventSwitchCameraMode3rd
  ;[1 1 1] Pick Up - Drop
  (Actor|Tick|SetActorTickEnabled false)
  (Components|Activation|Deactivate (Variables|Default|GetFollowCamera))
  (Components|Activation|Activate (Variables|Default|GetCameraComponent) false)
  (Class|PrimitiveComponent|SetOwnerNoSee (Variables|Character|GetMesh) false)
  (Variables|/Script/Engine.CharacterMovementComponent|SetMaxWalkSpeed (Variables|Character|GetCharacterMovement) 5e+02))

(event Input|ActionEvents|InputActionToggleCombatMode
  (params (Key :type Key%20Structure :default "None"))
  (bind _animationbp (Variables|Default|GetAnimationBP))
  ;[1 1 1] Damage/CombatMode/Stats
  (:Pressed
    (if (Variables|Default|GetDoesHaveWeapon)
      (if (not (Variables|Default|GetIsAttacking))
        (Utilities|FlowControl|FlipFlop
          (:A
            (Variables|/Game/Elf/CharacterAnimBP.CharacterAnimBP_C|SetIsInCombat _animationbp true)
            (Variables|/Game/Elf/CharacterAnimBP.CharacterAnimBP_C|SetIsUnHolstering _animationbp true)
            (Variables|Default|SetCombatMode true))
          (:B
            (Variables|Default|SetCombatMode false)
            (Variables|/Game/Elf/CharacterAnimBP.CharacterAnimBP_C|SetIsHolstering _animationbp true)))))))

(event Input|MouseEvents|RightMouseButton
  (params (Key :type Key%20Structure :default "None"))
  ;[1 1 1] Pick Up - Drop
  (:Pressed
    (if (Variables|Default|GetisHoldingObject)
      (CallFunction|Drop)
      (else
        (CallFunction|PickUp)))))

(event Input|MouseEvents|MouseWheelDown
  (params (Key :type Key%20Structure :default "None"))
  (bind _grablocation (Variables|Default|GetGrabLocation))
  (bind _relativelocation (Variables|/Script/Engine.SceneComponent|GetRelativeLocation _grablocation))
  ;[1 1 1] Pick Up - Drop
  (:Pressed
    (if (> (.x _relativelocation) 2.5e+02)
      (Transformation|SetRelativeLocation _grablocation (Math|Vector|MakeVector (+ (.x _relativelocation) -5e+01) (.y _relativelocation) (.z _relativelocation)) false true))))

(event Input|MouseEvents|MouseWheelUp
  (params (Key :type Key%20Structure :default "None"))
  (bind _grablocation (Variables|Default|GetGrabLocation))
  (bind _relativelocation (Variables|/Script/Engine.SceneComponent|GetRelativeLocation _grablocation))
  ;[1 1 1] Pick Up - Drop
  (:Pressed
    (if (< (.x _relativelocation) 3.5e+02)
      (Transformation|SetRelativeLocation _grablocation (Math|Vector|MakeVector (+ (.x _relativelocation) 5e+01) (.y _relativelocation) (.z _relativelocation)) false false))))

(event Input|MouseEvents|LeftMouseButton
  (params (Key :type Key%20Structure :default "None"))
  (bind _returnvalue (Game|GetPlayerCharacter 0))
  (bind _animationbp (Variables|Default|GetAnimationBP))
  (bind _returnvalue_2 (Transformation|GetActorLocation _returnvalue))
  ;[1 1 1] Damage/CombatMode/Stats
  (:Pressed
    (if (not (or (Variables|/Game/Elf/CharacterAnimBP.CharacterAnimBP_C|GetIsHolstering _animationbp) (Variables|/Game/Elf/CharacterAnimBP.CharacterAnimBP_C|GetIsUnHolstering _animationbp)))
      (if (Variables|Default|GetCombatMode)
        (if (not (Variables|Default|GetIsAttacking))
          (Variables|/Game/Elf/CharacterAnimBP.CharacterAnimBP_C|SetIsInAttackAnimation (Variables|Default|GetAnimationBP) true)
          (Variables|Default|SetIsAttacking true)
          (Variables|/Script/Engine.CharacterMovementComponent|SetMaxWalkSpeed (Variables|Character|GetCharacterMovement) 4.5e+02)
          (Utilities|FlowControl|Delay 0.4)
          (bind _outhit (Class|KismetSystemLibrary|BoxTraceSingleforObjects _returnvalue_2 (+ _returnvalue_2 (* (Transformation|GetActorForwardVector _returnvalue) 75)) "30.000000,50.000000,30.000000" (Transformation|GetActorRotation _returnvalue) (Variables|Default|GetObjTypes) false 0 "Persistent" true :!label _label))
          (Game|Damage|ApplyDamage (.HitActor (Collision|BreakHitResult _outhit)) 1.0 0 0)
          (bind _result (Math|Integer|IncrementInt (Variables|Default|GetCounter))
            (:%20%20
              (if (== _result 3)
                (Variables|Default|SetCounter 0)
                (else
                  (Utilities|FlowControl|Delay 0.2)
                  (goto _label))))))))))

(fn ConstructionScript)

(fn TakeDamageFunction
  (params (Amount :type Float%20%28single-precision%29))
  (Variables|Default|SetHealth (- (Variables|Default|GetHealth) Amount))
  (bind _foundwidgets (Widget|GetAllWidgetsOfClass "/Game/Elf/Stats/StatsWidget.StatsWidget_C" true))
  (Progress|SetPercent (Variables|/Game/Elf/Stats/StatsWidget.StatsWidget_C|GetHPBar (Utilities|Array|Get(acopy) _foundwidgets)) (Variables|Default|GetHealth)))