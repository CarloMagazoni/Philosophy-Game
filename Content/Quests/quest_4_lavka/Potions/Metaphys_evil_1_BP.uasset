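; Metaphys_evil_1_BP is an inspectable potion in the quest 4 shop (lavka) that gets a random bottle look and description.
; On BeginPlay it copies EvilExamples from row "3" of Evil_DataTable, picks one of two indices, and destroys all but one bottle component.
; The random roll never reaches the final branch, so Bottle5 is never kept.
; The Info event opens an Information_Widget showing the chosen example text.
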(event EventBeginPlay
  (bind _bottle1 (Variables|Default|Getbottle1))
  (Variables|Default|SetIndex (Math|Random|RandomIntegerinRange 4 5))
  (bind _returnvalue (Utilities|GetDataTableRow "/Game/Quests/quest_4_lavka/Potions/Evil_DataTable.Evil_DataTable" "3")
    (:then
      (for _array_element (.Evil_examples (Utilities|Struct|BreakEvil_struct _returnvalue))
        (Utilities|Array|Add (Variables|Default|GetEvil%20Examples) _array_element))
      (Variables|Default|Setbottle (Math|Random|RandomInteger 4))
      (if (== (Variables|Default|Getbottle) 0)
        (Components|DestroyComponent (Variables|Default|Getbottle5))
        (elif (== (Variables|Default|Getbottle) 1)
          (Components|DestroyComponent _bottle1)
          (elif (== (Variables|Default|Getbottle) 2)
            (Components|DestroyComponent _bottle1)
            (elif (== (Variables|Default|Getbottle) 3)
              (Components|DestroyComponent _bottle1)
              (else
                (Components|DestroyComponent _bottle1)))))))))

(event EventInfo
  (bind _returnvalue (UserInterface|CreateWidget "/Game/Entities/PickUp/Information_Widget.Information_Widget_C"))
  (UserInterface|Viewport|AddtoViewport _returnvalue 0)
  (Default|InspecttheObject _returnvalue (Utilities|String|ToString(Text) (Utilities|Array|Get(acopy) (Variables|Default|GetEvil%20Examples) (Variables|Default|GetIndex)))))

(fn ConstructionScript)