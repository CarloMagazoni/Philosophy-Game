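; Inspectable evil-morality object in the quest 4 potions content that shows a randomly chosen example of evil.
; On BeginPlay it rolls an index from a hard-coded range, independent of array length, and copies the examples from a fixed Evil_DataTable row.
; The Info event creates an Information_Widget, adds it to the viewport and passes it the chosen example, so the text stays the same until the next BeginPlay.
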(event EventInfo
  (bind _returnvalue (UserInterface|CreateWidget "/Game/Entities/PickUp/Information_Widget.Information_Widget_C"))
  (UserInterface|Viewport|AddtoViewport _returnvalue 0)
  (Default|InspecttheObject _returnvalue (Utilities|String|ToString(Text) (Utilities|Array|Get(acopy) (Variables|Default|GetEvil%20Examples) (Variables|Default|GetIndex)))))

(event EventBeginPlay
  (Variables|Default|SetIndex (Math|Random|RandomInteger 11))
  (bind _returnvalue (Utilities|GetDataTableRow "/Game/Quests/quest_4_lavka/Potions/Evil_DataTable.Evil_DataTable" "2")
    (:then
      (for _array_element (.Evil_examples (Utilities|Struct|BreakEvil_struct _returnvalue))
        (Utilities|Array|Add (Variables|Default|GetEvil%20Examples) _array_element)))))

(fn ConstructionScript)