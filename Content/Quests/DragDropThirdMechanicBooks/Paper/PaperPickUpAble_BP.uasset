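; Pickup paper page for the third-mechanic drag-and-drop books quest, collected with the Interact input.
; On BeginPlay it caches the first DragDropInteractableThirdMechanic in the level and notifies it that the page appeared.
; Its box overlap toggles input and a pickup widget for the player pawn.
; Interacting while near tells that owner the page was picked up, removes the widget and destroys the paper.
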(event OnComponentBeginOverlap(Box)
  (params (OverlappedComponent :type Primitive%20Component%20Object%20Reference) (OtherActor :type Actor%20Object%20Reference) (OtherComp :type Primitive%20Component%20Object%20Reference) (OtherBodyIndex :type Integer) (bFromSweep :type Boolean) (SweepResult :type Hit%20Result%20Structure%20%28by%20ref%29))
  (if (== OtherActor (Game|Player|GetPlayerPawn 0))
    (Variables|Default|SetIsNear true)
    (Input|EnableInput (Game|GetPlayerController 0))
    (if true
      (bind _returnvalue (UserInterface|CreateWidget "/Game/Quests/DragDropThirdMechanicBooks/Paper/PaperPickupAbleWidget.PaperPickupAbleWidget_C"))
      (bind _output_get (Variables|Default|SetPaperWidgetRef _returnvalue))
      (UserInterface|Viewport|AddtoViewport _output_get 0))))

(event OnComponentEndOverlap(Box)
  (params (OverlappedComponent :type Primitive%20Component%20Object%20Reference) (OtherActor :type Actor%20Object%20Reference) (OtherComp :type Primitive%20Component%20Object%20Reference) (OtherBodyIndex :type Integer))
  (if (== OtherActor (Game|Player|GetPlayerPawn 0))
    (Variables|Default|SetIsNear false)
    (Input|DisableInput (Game|GetPlayerController 0))
    (Widget|RemovefromParent (Variables|Default|GetPaperWidgetRef))))

(event EventBeginPlay
  (bind _outactors (Actor|GetAllActorsOfClass "/Game/Quests/DragDropThirdMechanicBooks/DragDropInteractableThirdMechanic.DragDropInteractableThirdMechanic_C"))
  (bind _output_get (Variables|Default|SetOwnerRef (Utilities|Array|Get(acopy) _outactors)))
  (Class|PaperandMechanicINTERF|OnPageAppear(Message) _output_get))

(event Input|ActionEvents|InputActionInteract
  (params (Key :type Key%20Structure :default "None"))
  (:Pressed
    (if (Variables|Default|GetIsNear)
      (Class|PaperandMechanicINTERF|OnPagePickUp(Message) (Variables|Default|GetOwnerRef))
      (Widget|RemovefromParent (Variables|Default|GetPaperWidgetRef))
      (Actor|DestroyActor))))

(fn ConstructionScript)