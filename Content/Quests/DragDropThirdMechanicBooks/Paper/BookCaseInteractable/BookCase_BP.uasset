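; BookCase_BP is a quest bookcase that can drop a paper pickup when the player walks into its box.
; On BeginPlay it finds the DragDropInteractableThirdMechanic actor and increments that actor's active bookcase count.
; The first player overlap disables the box and notifies that owner.
; A paper spawns above it on a coin flip, or always when the papers still missing from three equal the active bookcase count.
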(event OnComponentBeginOverlap(Box)
  (params (OverlappedComponent :type Primitive%20Component%20Object%20Reference) (OtherActor :type Actor%20Object%20Reference) (OtherComp :type Primitive%20Component%20Object%20Reference) (OtherBodyIndex :type Integer) (bFromSweep :type Boolean) (SweepResult :type Hit%20Result%20Structure%20%28by%20ref%29))
  (bind _ownerref (Variables|Default|GetOwnerRef))
  (if (== OtherActor (Game|Player|GetPlayerPawn 0))
    (Collision|SetCollisionEnabled (Variables|Default|GetBox) "NoCollision")
    (Class|PaperandMechanicINTERF|BookCaseUsed(Message) _ownerref)
    (if (== (- 3 (Variables|/Game/Quests/DragDropThirdMechanicBooks/DragDropInteractableThirdMechanic.DragDropInteractableThirdMechanic_C|GetPaperExisting _ownerref)) (Variables|/Game/Quests/DragDropThirdMechanicBooks/DragDropInteractableThirdMechanic.DragDropInteractableThirdMechanic_C|GetBookCasesActive _ownerref))
      (Game|SpawnActorfromClass "/Game/Quests/DragDropThirdMechanicBooks/Paper/PaperPickUpAble_BP.PaperPickUpAble_BP_C" (Math|Transform|MakeTransform (+ (Transformation|GetActorLocation) "0, 0,50.000000") "0, 0, 0" "1,1,1") "Undefined" 0 0 :!label _label)
      (elif (Math|Random|RandomBool)
        (goto _label)))))

(event EventBeginPlay
  (bind _outactors (Actor|GetAllActorsOfClass "/Game/Quests/DragDropThirdMechanicBooks/DragDropInteractableThirdMechanic.DragDropInteractableThirdMechanic_C"))
  (bind _output_get (Variables|Default|SetOwnerRef (Utilities|Array|Get(acopy) _outactors)))
  (Math|Integer|IncrementInt (Variables|/Game/Quests/DragDropThirdMechanicBooks/DragDropInteractableThirdMechanic.DragDropInteractableThirdMechanic_C|GetBookCasesActive _output_get)))

(fn ConstructionScript)