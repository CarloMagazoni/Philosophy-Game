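; Neutral potion prop for the shop quest that keeps one random bottle mesh out of five and carries a random neutral example text.
; BeginPlay places all bottles at Position, gathers NeutralExamples from Evil_DataTable rows, picks an index and destroys the unused bottles.
; Restart teleports the surviving bottle back to Position, and Info shows its text in an Information_Widget.
; Hard hits play a debounced glass sound, with a separate impulse threshold per bottle.
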(event OnComponentHit(bottle5)
  (params (HitComponent :type Primitive%20Component%20Object%20Reference) (OtherActor :type Actor%20Object%20Reference) (OtherComp :type Primitive%20Component%20Object%20Reference) (NormalImpulse :type Vector :default "0, 0, 0") (Hit :type Hit%20Result%20Structure%20%28by%20ref%29))
  (if (>= (Math|Vector|VectorLength NormalImpulse) 1.33e+03)
    (Utilities|FlowControl|DoOnce false :!label _label
      (:Completed
        (Audio|PlaySound2D "/Game/Sounds/SFX_general/glass/glass_Cue.glass_Cue" 1.0 1.0 0.0 0 0)
        (Utilities|FlowControl|Delay 0.2)
        (goto _label Reset)))))

(event OnComponentHit(bottle2)
  (params (HitComponent :type Primitive%20Component%20Object%20Reference) (OtherActor :type Actor%20Object%20Reference) (OtherComp :type Primitive%20Component%20Object%20Reference) (NormalImpulse :type Vector :default "0, 0, 0") (Hit :type Hit%20Result%20Structure%20%28by%20ref%29))
  (if (>= (Math|Vector|VectorLength NormalImpulse) 1.18e+03)
    (Utilities|FlowControl|DoOnce false :!label _label
      (:Completed
        (Audio|PlaySound2D "/Game/Sounds/SFX_general/glass/glass_Cue.glass_Cue" 1.0 1.0 0.0 0 0)
        (Utilities|FlowControl|Delay 0.2)
        (goto _label Reset)))))

(event OnComponentHit(bottle4)
  (params (HitComponent :type Primitive%20Component%20Object%20Reference) (OtherActor :type Actor%20Object%20Reference) (OtherComp :type Primitive%20Component%20Object%20Reference) (NormalImpulse :type Vector :default "0, 0, 0") (Hit :type Hit%20Result%20Structure%20%28by%20ref%29))
  (if (>= (Math|Vector|VectorLength NormalImpulse) 1.7e+03)
    (Utilities|FlowControl|DoOnce false :!label _label
      (:Completed
        (Audio|PlaySound2D "/Game/Sounds/SFX_general/glass/glass_Cue.glass_Cue" 1.0 1.0 0.0 0 0)
        (Utilities|FlowControl|Delay 0.2)
        (goto _label Reset)))))

(event OnComponentHit(bottle1)
  (params (HitComponent :type Primitive%20Component%20Object%20Reference) (OtherActor :type Actor%20Object%20Reference) (OtherComp :type Primitive%20Component%20Object%20Reference) (NormalImpulse :type Vector :default "0, 0, 0") (Hit :type Hit%20Result%20Structure%20%28by%20ref%29))
  (if (>= (Math|Vector|VectorLength NormalImpulse) 2.8e+02)
    (Utilities|FlowControl|DoOnce false :!label _label
      (:Completed
        (Audio|PlaySound2D "/Game/Sounds/SFX_general/glass/glass_Cue.glass_Cue" 1.0 1.0 0.0 0 0)
        (Utilities|FlowControl|Delay 0.2)
        (goto _label Reset)))))

(event OnComponentHit(bottle3)
  (params (HitComponent :type Primitive%20Component%20Object%20Reference) (OtherActor :type Actor%20Object%20Reference) (OtherComp :type Primitive%20Component%20Object%20Reference) (NormalImpulse :type Vector :default "0, 0, 0") (Hit :type Hit%20Result%20Structure%20%28by%20ref%29))
  (if (>= (Math|Vector|VectorLength NormalImpulse) 4e+02)
    (Utilities|FlowControl|DoOnce false :!label _label
      (:Completed
        (Audio|PlaySound2D "/Game/Sounds/SFX_general/glass/glass_Cue.glass_Cue" 1.0 1.0 0.0 0 0)
        (Utilities|FlowControl|Delay 0.2)
        (goto _label Reset)))))

(event EventRestart
  (bind _bottle (Variables|Default|Getbottle))
  (if (== _bottle 0)
    (Transformation|SetWorldLocation (Variables|Default|Getbottle1) (Variables|Default|GetPosition) false true)
    (elif (== _bottle 1)
      (Transformation|SetWorldLocation (Variables|Default|Getbottle2) (Variables|Default|GetPosition) false true)
      (elif (== _bottle 2)
        (Transformation|SetWorldLocation (Variables|Default|Getbottle3) (Variables|Default|GetPosition) false true)
        (elif (== _bottle 3)
          (Transformation|SetWorldLocation (Variables|Default|Getbottle4) (Variables|Default|GetPosition) false true)
          (else
            (Transformation|SetWorldLocation (Variables|Default|Getbottle5) (Variables|Default|GetPosition) false true)))))))

(event EventBeginPlay
  (bind _bottle1 (Variables|Default|Getbottle1))
  (Utilities|FlowControl|Delay 0.2)
  (Transformation|SetWorldLocation (Variables|Default|Getbottle1) (Variables|Default|GetPosition) false true)
  (bind _outrownames (DataTable|GetDataTableRowNames "/Game/Quests/quest_3_lavka/Potions/Evil_DataTable.Evil_DataTable"))
  (for _array_element _outrownames
    (bind _returnvalue (Utilities|GetDataTableRow "/Game/Quests/quest_3_lavka/Potions/Evil_DataTable.Evil_DataTable" _array_element)
      (:then
        (for _array_element_2 (.Neutral_examples (Utilities|Struct|BreakEvil_struct _returnvalue))
          (Utilities|Array|Add (Variables|Default|GetNeutral%20Examples) _array_element_2)))))
  (Variables|Default|SetIndex (Math|Random|RandomIntegerinRange 0 8))
  (Variables|Default|Setbottle (Math|Random|RandomInteger 5))
  (if (== (Variables|Default|Getbottle) 0)
    (Components|DestroyComponent (Variables|Default|Getbottle5))
    (elif (== (Variables|Default|Getbottle) 1)
      (Components|DestroyComponent _bottle1)
      (elif (== (Variables|Default|Getbottle) 2)
        (Components|DestroyComponent _bottle1)
        (elif (== (Variables|Default|Getbottle) 3)
          (Components|DestroyComponent _bottle1)
          (else
            (Components|DestroyComponent _bottle1)))))))

(event EventInfo
  (bind _returnvalue (UserInterface|CreateWidget "/Game/Entities/PickUp/Information_Widget.Information_Widget_C"))
  (UserInterface|Viewport|AddtoViewport _returnvalue 0)
  (Default|InspecttheObject _returnvalue (Utilities|String|ToString(Text) (Utilities|Array|Get(acopy) (Variables|Default|GetNeutral%20Examples) (Variables|Default|GetIndex)))))

(fn ConstructionScript)