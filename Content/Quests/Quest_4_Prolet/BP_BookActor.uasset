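; Interactable book actor for the Prolet quest that opens a reading or quest UI when the player presses Interact nearby.
; The Rt overlap toggles input and, when GameInstance quest flags allow, a pickup prompt, using paired DoOnce gates that reset each other.
; Interact hides visible quest info, then opens either the paused Book_quest3 screen or WPB_Book with its Prolet message and dialogue state, in UI-only input.
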(event OnComponentBeginOverlap(rt)
  (params (OverlappedComponent :type Primitive%20Component%20Object%20Reference) (OtherActor :type Actor%20Object%20Reference) (OtherComp :type Primitive%20Component%20Object%20Reference) (OtherBodyIndex :type Integer) (bFromSweep :type Boolean) (SweepResult :type Hit%20Result%20Structure%20%28by%20ref%29))
  (Input|EnableInput (Game|GetPlayerController 0))
  (bind _asmy_gi (Utilities|Casting|CastToMyGI (Game|GetGameInstance)))
  (if (Variables|/Game/Quests/Quest_4_Prolet/MyGI.MyGI_C|GetmustGoToBook_3_quest_lavka _asmy_gi)
    (Utilities|FlowControl|DoOnce false :!label _label
      (:Completed
        (bind _returnvalue (UserInterface|CreateWidget "/Game/Quests/Quest_4_Prolet/PickUp_Widget_Prolet.PickUp_Widget_Prolet_C"))
        (UserInterface|Viewport|AddtoViewport _returnvalue 0)
        (Utilities|FlowControl|DoOnce false) ; enters at Reset
      ))
    (elif (Variables|/Game/Quests/Quest_4_Prolet/MyGI.MyGI_C|GetcanReadBook _asmy_gi)
      (goto _label))))

(event OnComponentEndOverlap(rt)
  (params (OverlappedComponent :type Primitive%20Component%20Object%20Reference) (OtherActor :type Actor%20Object%20Reference) (OtherComp :type Primitive%20Component%20Object%20Reference) (OtherBodyIndex :type Integer))
  (Input|DisableInput (Game|GetPlayerController 0))
  (bind _asmy_gi (Utilities|Casting|CastToMyGI (Game|GetGameInstance)))
  (if (Variables|/Game/Quests/Quest_4_Prolet/MyGI.MyGI_C|GetmustGoToBook_3_quest_lavka _asmy_gi)
    (Utilities|FlowControl|DoOnce false :!label _label
      (:Completed
        (UserInterface|Animation|PlayAnimation (stale OnComponentBeginOverlap(rt) _returnvalue) (Variables|/Game/Quests/Quest_4_Prolet/PickUp_Widget_Prolet.PickUp_Widget_Prolet_C|GetPickUp_FadeOut (stale OnComponentBeginOverlap(rt) _returnvalue)) 0.0 1 "Forward" 1.0 false)
        (Utilities|FlowControl|Delay 0.45)
        (Widget|RemovefromParent (stale OnComponentBeginOverlap(rt) _returnvalue))
        (Utilities|FlowControl|DoOnce false) ; enters at Reset
      ))
    (elif (Variables|/Game/Quests/Quest_4_Prolet/MyGI.MyGI_C|GetcanReadBook _asmy_gi)
      (goto _label))))

(event EventForBook
  (params (Prolet :type Integer))
  (Variables|Default|Setprolet Prolet))

(event Input|ActionEvents|InputActionInteract
  (params (Key :type Key%20Structure :default "None"))
  (bind _returnvalue (Game|GetPlayerController 0))
  (:Pressed
    (bind _asmy_gi (Utilities|Casting|CastToMyGI (Game|GetGameInstance)))
    (if (Variables|/Game/Quests/Quest_4_Prolet/MyGI.MyGI_C|GetmustGoToBook_3_quest_lavka _asmy_gi)
      (bind _foundwidgets (Widget|GetAllWidgetsOfClass "/Game/GameQuestWidgets/QuestInfo.QuestInfo_C" true))
      (if (Variables|/Game/GameQuestWidgets/QuestInfo.QuestInfo_C|GetVisible (Utilities|Array|Get(acopy) _foundwidgets))
        (Class|QuestInfoShowonOff|On/Off(Message) _foundwidgets))
      (bind _returnvalue_2 (UserInterface|CreateWidget "/Game/Quests/quest_3_lavka/Book/book_quest3.book_quest3_C"))
      (UserInterface|Viewport|AddtoViewport _returnvalue_2 0)
      (Game|SetGamePaused true)
      (Input|SetInputModeUIOnly _returnvalue _returnvalue_2 "DoNotLock")
      (Variables|/Script/Engine.PlayerController|SetbShowMouseCursor _returnvalue true)
      (Utilities|FlowControl|DoOnce false :!label _label
        (:Completed
          (UserInterface|Animation|PlayAnimation (stale OnComponentBeginOverlap(rt) _returnvalue) (Variables|/Game/Quests/Quest_4_Prolet/PickUp_Widget_Prolet.PickUp_Widget_Prolet_C|GetPickUp_FadeOut (stale OnComponentBeginOverlap(rt) _returnvalue)) 0.0 1 "Forward" 1.0 false)
          (Utilities|FlowControl|Delay 0.45)
          (Widget|RemovefromParent (stale OnComponentBeginOverlap(rt) _returnvalue))
          (Utilities|FlowControl|DoOnce false) ; enters at Reset
        ))
      (elif (Variables|/Game/Quests/Quest_4_Prolet/MyGI.MyGI_C|GetcanReadBook _asmy_gi)
        (bind _foundwidgets_2 (Widget|GetAllWidgetsOfClass "/Game/GameQuestWidgets/QuestInfo.QuestInfo_C" true))
        (if (Variables|/Game/GameQuestWidgets/QuestInfo.QuestInfo_C|GetVisible (Utilities|Array|Get(acopy) _foundwidgets_2))
          (Class|QuestInfoShowonOff|On/Off(Message) _foundwidgets_2))
        (bind _returnvalue_3 (UserInterface|CreateWidget "/Game/Quests/Quest_4_Prolet/WPB_Book.WPB_Book_C"))
        (UserInterface|Viewport|AddtoViewport _returnvalue_3 0)
        (Class|BPIStairs|ForBook(Message) _returnvalue_3 (Variables|Default|Getprolet))
        (Variables|/Script/PhilosophyProject.PlayableCharacter|SetInDialogue (.AsBP%20Playable%20Character (Utilities|Casting|CastToBP_PlayableCharacter (Game|GetPlayerCharacter 0))) true)
        (Input|SetInputModeUIOnly _returnvalue _returnvalue_3 "DoNotLock")
        (Variables|/Script/Engine.PlayerController|SetbShowMouseCursor _returnvalue true)
        (goto _label)))))

(fn ConstructionScript)