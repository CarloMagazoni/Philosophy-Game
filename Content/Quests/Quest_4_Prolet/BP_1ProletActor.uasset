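; BP_1ProletActor is a quest trigger actor for the Prolet quest that opens the WBP_1Prolet widget when its Re component is overlapped.
; It only fires once started and not yet passed, and gates on the game instance's Mistake count, requiring a read book or a fountain visit after mistakes.
; The widget takes UI-only input with a cursor, then the game pauses after a short delay.
; ForProlet sets the passed flag and destroys the Plane component.
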(event OnComponentBeginOverlap(re)
  (params (OverlappedComponent :type Primitive%20Component%20Object%20Reference) (OtherActor :type Actor%20Object%20Reference) (OtherComp :type Primitive%20Component%20Object%20Reference) (OtherBodyIndex :type Integer) (bFromSweep :type Boolean) (SweepResult :type Hit%20Result%20Structure%20%28by%20ref%29))
  (bind _returnvalue (Game|GetPlayerController 0))
  (if (Variables|Default|Getstarted)
    (if (not (Variables|Default|Getprolet))
      (bind _asmy_gi (Utilities|Casting|CastToMyGI (Game|GetGameInstance)))
      (if (== (Variables|/Game/Quests/Quest_4_Prolet/MyGI.MyGI_C|GetMistake _asmy_gi) 0)
        (bind _returnvalue_2 (UserInterface|CreateWidget "/Game/Quests/Quest_4_Prolet/WBP_1Prolet.WBP_1Prolet_C" :!label _label))
        (UserInterface|Viewport|AddtoViewport _returnvalue_2 0)
        (Input|SetInputModeUIOnly _returnvalue 0 "DoNotLock")
        (Variables|/Script/Engine.PlayerController|SetbShowMouseCursor _returnvalue true)
        (Utilities|FlowControl|Delay 0.1)
        (Game|SetGamePaused true)
        (elif (== (Variables|/Game/Quests/Quest_4_Prolet/MyGI.MyGI_C|GetMistake _asmy_gi) 1)
          (if (Variables|/Game/Quests/Quest_4_Prolet/MyGI.MyGI_C|GethadReadBook _asmy_gi)
            (goto _label))
          (elif (== (Variables|/Game/Quests/Quest_4_Prolet/MyGI.MyGI_C|GetMistake _asmy_gi) 2)
            (if (Variables|/Game/Quests/Quest_4_Prolet/MyGI.MyGI_C|GethadGoneToFontan _asmy_gi)
              (goto _label))))))))

(event EventForProlet
  (params (Prolet :type Boolean))
  (Variables|Default|Setprolet Prolet)
  (Components|DestroyComponent (Variables|Default|GetPlane)))

(fn ConstructionScript)