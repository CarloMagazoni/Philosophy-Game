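; Big fountain actor that the player can interact with while standing inside its sphere trigger.
; Sphere overlap toggles the proximity flag and the actor's input.
; Interact, when the player is near and IsFail is set, finds the Zasovs actor and sets its IsTestValible flag to true.
; A drink sequence with camera blend, input lock and montage is left disconnected and never runs.
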(event OnComponentBeginOverlap(Sphere)
  (params (OverlappedComponent :type Primitive%20Component%20Object%20Reference) (OtherActor :type Actor%20Object%20Reference) (OtherComp :type Primitive%20Component%20Object%20Reference) (OtherBodyIndex :type Integer) (bFromSweep :type Boolean) (SweepResult :type Hit%20Result%20Structure%20%28by%20ref%29))
  ;[0.9583 0.7261 0.3322 0.575] is player near
  (Variables|Default|SetisPlayerNear true)
  (Input|EnableInput (Game|GetPlayerController 0)))

(event OnComponentEndOverlap(Sphere)
  (params (OverlappedComponent :type Primitive%20Component%20Object%20Reference) (OtherActor :type Actor%20Object%20Reference) (OtherComp :type Primitive%20Component%20Object%20Reference) (OtherBodyIndex :type Integer))
  ;[0.9583 0.7261 0.3322 0.575] is player near
  (Variables|Default|SetisPlayerNear false)
  (Input|DisableInput (Game|GetPlayerController 0)))

(event Input|ActionEvents|InputActionInteract
  (params (Key :type Key%20Structure :default "None"))
  ;[0 0.441 1] drink Animation
  (:Pressed
    (if (and (Variables|Default|GetisPlayerNear) (Variables|Default|GetisFail))
      (bind _returnvalue (Actor|GetActorOfClass "/Game/Quests/quest_5_gate/zasovs.zasovs_C"))
      (Variables|/Game/Quests/quest_5_gate/zasovs.zasovs_C|SetisTestValible _returnvalue true))))

(fn ConstructionScript)