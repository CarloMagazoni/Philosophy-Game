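; Interactable fountain that lets the player drink once IsFail is set, playing a sound and montage from a cinematic camera.
; An overlap sphere toggles input and the PressToDrink prompt.
; On Interact, the camera orbits the fountain center using angle and rotation offsets cached at BeginPlay from a GgModel reference, reproducing the framing wherever the player stands.
; Afterwards it restores the view, shows Widget_Udrink, flags IsTestValible on Zasovs and clears IsFail.
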(event OnComponentBeginOverlap(Sphere)
  (params (OverlappedComponent :type Primitive%20Component%20Object%20Reference) (OtherActor :type Actor%20Object%20Reference) (OtherComp :type Primitive%20Component%20Object%20Reference) (OtherBodyIndex :type Integer) (bFromSweep :type Boolean) (SweepResult :type Hit%20Result%20Structure%20%28by%20ref%29))
  ;[0.9583 0.7261 0.3322 0.575] is player near
  (Variables|Default|SetisPlayerNear true)
  (Input|EnableInput (Game|GetPlayerController 0))
  (if (Variables|Default|GetisFail)
    (bind _returnvalue (UserInterface|CreateWidget "/Game/Quests/quest_5_gate/fountain/pressToDrink.pressToDrink_C"))
    (UserInterface|Viewport|AddtoViewport _returnvalue 0)))

(event OnComponentEndOverlap(Sphere)
  (params (OverlappedComponent :type Primitive%20Component%20Object%20Reference) (OtherActor :type Actor%20Object%20Reference) (OtherComp :type Primitive%20Component%20Object%20Reference) (OtherBodyIndex :type Integer))
  ;[0.9583 0.7261 0.3322 0.575] is player near
  (Variables|Default|SetisPlayerNear false)
  (Input|DisableInput (Game|GetPlayerController 0))
  (bind _foundwidgets (Widget|GetAllWidgetsOfClass "/Game/Quests/quest_5_gate/fountain/pressToDrink.pressToDrink_C" true))
  (Widget|RemovefromParent _foundwidgets))

(event EventBeginPlay
  (bind _camera (Variables|Default|GetCamera))
  (bind _camera_2 (Variables|Default|GetCamera))
  (bind _returnvalue (Transformation|GetWorldRotation _camera_2))
  (bind _returnvalue_2 (Transformation|GetWorldLocation _camera))
  ;[1 0.9818 0.1829] set constans
  (Variables|Default|Setoriginal_gg_coordinates (Transformation|GetWorldLocation (Variables|Default|Getgg_model)))
  (bind _output_get (Variables|Default|Setfountain_center (Transformation|GetWorldLocation (Variables|Default|GetPlane))))
  (Variables|Default|Setoriginal_camera_vector (Math|Vector|MakeVector (- (.x _output_get) (.x _returnvalue_2)) (- (.y _output_get) (.y _returnvalue_2)) 0.0))
  (Variables|Default|Setcamera_radius (Math|Float|Sqrt (+ (Math|Float|Square (- (.x _output_get) (.x _returnvalue_2))) (Math|Float|Square (- (.y _output_get) (.y _returnvalue_2))))))
  (Variables|Default|Setcamera_angle (* -1 (Math|Trig|Acos(Degrees) (/ (+ (* (- (.x (Variables|Default|Getfountain_center)) (.x (Variables|Default|Getoriginal_gg_coordinates))) (.x (Variables|Default|Getoriginal_camera_vector))) (* (- (.y (Variables|Default|Getfountain_center)) (.y (Variables|Default|Getoriginal_gg_coordinates))) (.y (Variables|Default|Getoriginal_camera_vector)))) (* (Math|Float|Sqrt (+ (Math|Float|Square (- (.x (Variables|Default|Getfountain_center)) (.x (Variables|Default|Getoriginal_gg_coordinates)))) (Math|Float|Square (- (.y (Variables|Default|Getfountain_center)) (.y (Variables|Default|Getoriginal_gg_coordinates)))))) (Math|Float|Sqrt (+ (Math|Float|Square (.x (Variables|Default|Getoriginal_camera_vector))) (Math|Float|Square (.y (Variables|Default|Getoriginal_camera_vector))))))))))
  (Variables|Default|Setx_rotation (- (.roll _returnvalue) (.roll (Math|Rotator|FindLookatRotation (Transformation|GetWorldLocation _camera_2) (Variables|Default|Getoriginal_gg_coordinates)))))
  (Variables|Default|Sety_rotation (- (.pitch _returnvalue) (.pitch (Math|Rotator|FindLookatRotation (Transformation|GetWorldLocation _camera_2) (Variables|Default|Getoriginal_gg_coordinates)))))
  (Variables|Default|Setz_rotation (- (.yaw _returnvalue) (.yaw (Math|Rotator|FindLookatRotation (Transformation|GetWorldLocation _camera_2) (Variables|Default|Getoriginal_gg_coordinates))))))

(event Input|ActionEvents|InputActionInteract
  (params (Key :type Key%20Structure :default "None"))
  (bind _returnvalue (Game|GetPlayerCharacter 0))
  (bind _returnvalue_2 (Game|GetPlayerCharacter 0))
  (bind _returnvalue_3 (Game|GetPlayerController 0))
  (bind _returnvalue_4 (Pawn|GetController _returnvalue_2))
  (bind _returnvalue_5 (Pawn|GetControlRotation _returnvalue_4 :!class /Script/Engine.Controller))
  ;[0 0.441 1] drink Animation
  (:Pressed
    (if (and (Variables|Default|GetisPlayerNear) (Variables|Default|GetisFail))
      (Audio|PlaySound2D "/Game/Sounds/SFX_general/drinking_Cue.drinking_Cue" 1.0 1.0 0.0 0 0)
      (Pawn|SetControlRotation _returnvalue_4 (Math|Rotator|MakeRotator (.roll _returnvalue_5) (.pitch _returnvalue_5) (.Yaw (Math|Rotator|BreakRotator (Math|Rotator|FindLookatRotation (Transformation|GetActorLocation _returnvalue_2) (Transformation|GetActorLocation))))))
      (CallFunction|ChangeCameraLocation)
      (CallFunction|ChangeCameraRotation)
      (bind _foundwidgets (Widget|GetAllWidgetsOfClass "/Game/Quests/quest_5_gate/fountain/pressToDrink.pressToDrink_C" true))
      (Widget|RemovefromParent _foundwidgets)
      (Game|Player|SetViewTargetwithBlend (Game|GetPlayerController 0) self 0.0 "VTBlend_Linear" 0.0 false)
      (Input|DisableInput _returnvalue _returnvalue_3)
      (bind _returnvalue_6 (Animation|PlayAnimMontage _returnvalue "/Game/Quests/quest_5_gate/fountain/drinking_montage.drinking_montage" 1.0 "None"))
      (Utilities|FlowControl|Delay _returnvalue_6)
      (Game|Player|SetViewTargetwithBlend _returnvalue_3 _returnvalue 0.0 "VTBlend_Linear" 0.0 false)
      (bind _returnvalue_7 (UserInterface|CreateWidget "/Game/Quests/quest_5_gate/fountain/Widget_Udrink.Widget_Udrink_C"))
      (Input|SetInputModeUIOnly _returnvalue_3 0 "DoNotLock")
      (UserInterface|Viewport|AddtoViewport _returnvalue_7 0)
      (Variables|/Script/Engine.PlayerController|SetbShowMouseCursor _returnvalue_3 true)
      (bind _returnvalue_8 (Actor|GetActorOfClass "/Game/Quests/quest_5_gate/zasovs_Auto1.zasovs_C"))
      (Variables|/Game/Quests/quest_5_gate/zasovs_Auto1.zasovs_C|SetisTestValible _returnvalue_8 true)
      (Variables|Default|SetisFail false))))

(fn ConstructionScript)

(fn ChangeCameraRotation
  (bind _returnvalue (Game|GetPlayerCharacter 0))
  (bind _camera (Variables|Default|GetCamera))
  (bind _returnvalue_2 (Transformation|GetWorldLocation _camera))
  (bind _returnvalue_3 (Transformation|GetActorLocation _returnvalue))
  (bind _returnvalue_4 (Math|Rotator|FindLookatRotation _returnvalue_2 _returnvalue_3))
  (Transformation|SetWorldRotation (Variables|Default|GetCamera) (Math|Rotator|MakeRotator (+ (.roll _returnvalue_4) (Variables|Default|Getx_rotation)) (+ (.pitch _returnvalue_4) (Variables|Default|Gety_rotation)) (+ (.yaw _returnvalue_4) (Variables|Default|Getz_rotation))) false false)
  (return))

(fn ChangeCameraLocation
  (bind _returnvalue (Game|GetPlayerCharacter 0))
  (bind _camera_radius (Variables|Default|Getcamera_radius))
  (bind _fountain_center (Variables|Default|Getfountain_center))
  (bind _fountain_center_2 (Variables|Default|Getfountain_center))
  (bind _fountain_center_3 (Variables|Default|Getfountain_center))
  (bind _fountain_center_4 (Variables|Default|Getfountain_center))
  (bind _returnvalue_2 (Transformation|GetActorLocation _returnvalue))
  (bind _returnvalue_3 (- (.y _returnvalue_2) (.y _fountain_center_4)))
  (bind _returnvalue_4 (- (.x _returnvalue_2) (.x _fountain_center_4)))
  (bind _returnvalue_5 (Math|Float|Square _returnvalue_4))
  (bind _returnvalue_6 (Math|Float|Square _returnvalue_3))
  (bind _returnvalue_7 (+ _returnvalue_5 _returnvalue_6))
  (bind _returnvalue_8 (Math|Float|Sqrt _returnvalue_7))
  (bind _returnvalue_9 (/ _camera_radius _returnvalue_8))
  (bind _output_get (LocalVariables|Setgg_circle_location (Math|Vector|MakeVector (+ (* _returnvalue_4 _returnvalue_9) (.x _fountain_center_3)) (+ (* _returnvalue_9 _returnvalue_3) (.y _fountain_center_3)) 0.0)))
  (Transformation|SetWorldLocation (Variables|Default|GetCamera) (Math|Vector|MakeVector (- (+ (* (- (.x _output_get) (.x _fountain_center)) (Math|Trig|Cos(Radians) (Variables|Default|Getcamera_angle))) (.x _fountain_center)) (* (- (.y _output_get) (.y _fountain_center)) (Math|Trig|Sin(Radians) (Variables|Default|Getcamera_angle)))) (+ (+ (* (- (.x (LocalVariables|Getgg_circle_location)) (.x _fountain_center_2)) (Math|Trig|Sin(Radians) (Variables|Default|Getcamera_angle))) (.y _fountain_center_2)) (* (- (.y (LocalVariables|Getgg_circle_location)) (.y _fountain_center_2)) (Math|Trig|Cos(Radians) (Variables|Default|Getcamera_angle)))) (.z (Transformation|GetWorldLocation (Variables|Default|GetCamera)))) false false)
  (return))