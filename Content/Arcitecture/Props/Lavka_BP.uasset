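; Lavka shop prop running a sorting puzzle: the player must place nine tagged objects into Phys, Moral and Metaphys evil trigger zones.
; Entering the input trigger raises invisible walls, switches to FPS camera, enables input and first shows a paused controls widget, reopenable with V.
; Overlaps track per-object flags; pressing C drops any held object and checks them.
; Success releases the player; failure also blocks retries until NewTryLavka, flags the game instance and escalates failure widgets.
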(event OnComponentBeginOverlap(Phys)
  (params (OverlappedComponent :type Primitive%20Component%20Object%20Reference) (OtherActor :type Actor%20Object%20Reference) (OtherComp :type Primitive%20Component%20Object%20Reference) (OtherBodyIndex :type Integer) (bFromSweep :type Boolean) (SweepResult :type Hit%20Result%20Structure%20%28by%20ref%29))
  (if (Actor|ActorHasTag OtherActor "Phys_1")
    (Variables|Default|SetPhys_evil_1 true)
    (Development|PrintString "Hello" :!label _label)
    (elif (Actor|ActorHasTag OtherActor "Phys_2")
      (Variables|Default|SetPhys_evil_2 true)
      (goto _label)
      (elif (Actor|ActorHasTag OtherActor "Phys_3")
        (Variables|Default|SetPhys_evil_3 true)
        (goto _label)))))

(event OnComponentBeginOverlap(Moral)
  (params (OverlappedComponent :type Primitive%20Component%20Object%20Reference) (OtherActor :type Actor%20Object%20Reference) (OtherComp :type Primitive%20Component%20Object%20Reference) (OtherBodyIndex :type Integer) (bFromSweep :type Boolean) (SweepResult :type Hit%20Result%20Structure%20%28by%20ref%29))
  (if (Actor|ActorHasTag OtherActor "Moral_1")
    (Variables|Default|SetMoral_evil_1 true)
    (Development|PrintString "Hello" :!label _label)
    (elif (Actor|ActorHasTag OtherActor "Moral_2")
      (Variables|Default|SetMoral_evil_2 true)
      (goto _label)
      (elif (Actor|ActorHasTag OtherActor "Moral_3")
        (Variables|Default|SetMoral_evil_3 true)
        (goto _label)))))

(event OnComponentBeginOverlap(Metaphys)
  (params (OverlappedComponent :type Primitive%20Component%20Object%20Reference) (OtherActor :type Actor%20Object%20Reference) (OtherComp :type Primitive%20Component%20Object%20Reference) (OtherBodyIndex :type Integer) (bFromSweep :type Boolean) (SweepResult :type Hit%20Result%20Structure%20%28by%20ref%29))
  (if (Actor|ActorHasTag OtherActor "Metaphys_1")
    (Variables|Default|SetMetaphys_evil_1 true)
    (Development|PrintString "Hello" :!label _label)
    (elif (Actor|ActorHasTag OtherActor "Metaphys_2")
      (Variables|Default|SetMetaphys_evil_2 true)
      (goto _label)
      (elif (Actor|ActorHasTag OtherActor "Metaphys_3")
        (Variables|Default|SetMetaphys_evil_3 true)
        (goto _label)))))

(event OnComponentBeginOverlap(Input_enable)
  (params (OverlappedComponent :type Primitive%20Component%20Object%20Reference) (OtherActor :type Actor%20Object%20Reference) (OtherComp :type Primitive%20Component%20Object%20Reference) (OtherBodyIndex :type Integer) (bFromSweep :type Boolean) (SweepResult :type Hit%20Result%20Structure%20%28by%20ref%29))
  (bind _returnvalue (Game|GetPlayerController 0))
  (if (Variables|Default|GetCan_try)
    (Utilities|FlowControl|Sequence
      (:then_0
        (Utilities|FlowControl|DoOnce false
          (:Completed
            (Utilities|FlowControl|Delay 0.1)
            (Game|SetGamePaused true)
            (bind _returnvalue_2 (UserInterface|CreateWidget "/Game/Quests/quest_3_lavka/Book/Lavka_controls_widget.Lavka_controls_widget_C"))
            (UserInterface|Viewport|AddtoViewport _returnvalue_2 0)
            (Input|SetInputModeUIOnly _returnvalue _returnvalue_2 "DoNotLock")
            (Variables|/Script/Engine.PlayerController|SetbShowMouseCursor _returnvalue true))))
      (:then_1
        (Input|EnableInput (Game|GetPlayerController 0))
        (Collision|SetCollisionEnabled (Variables|Default|GetInv_wall_1) "QueryAndPhysics")
        (Class|SwitchCameraModeFps|SwitchCameraModeFps(Message) (Game|GetPlayerCharacter 0))))))

(event OnComponentEndOverlap(Phys)
  (params (OverlappedComponent :type Primitive%20Component%20Object%20Reference) (OtherActor :type Actor%20Object%20Reference) (OtherComp :type Primitive%20Component%20Object%20Reference) (OtherBodyIndex :type Integer))
  (if (Actor|ActorHasTag OtherActor "Phys_1")
    (Variables|Default|SetPhys_evil_1 false)
    (Development|PrintString "Hello" :!label _label)
    (elif (Actor|ActorHasTag OtherActor "Phys_2")
      (Variables|Default|SetPhys_evil_2 false)
      (goto _label)
      (elif (Actor|ActorHasTag OtherActor "Phys_3")
        (Variables|Default|SetPhys_evil_3 false)
        (goto _label)))))

(event OnComponentEndOverlap(Moral)
  (params (OverlappedComponent :type Primitive%20Component%20Object%20Reference) (OtherActor :type Actor%20Object%20Reference) (OtherComp :type Primitive%20Component%20Object%20Reference) (OtherBodyIndex :type Integer))
  (if (Actor|ActorHasTag OtherActor "Moral_1")
    (Variables|Default|SetMoral_evil_1 false)
    (Development|PrintString "Hello" :!label _label)
    (elif (Actor|ActorHasTag OtherActor "Moral_2")
      (Variables|Default|SetMoral_evil_2 false)
      (goto _label)
      (elif (Actor|ActorHasTag OtherActor "Moral_3")
        (Variables|Default|SetMoral_evil_3 false)
        (goto _label)))))

(event OnComponentEndOverlap(Metaphys)
  (params (OverlappedComponent :type Primitive%20Component%20Object%20Reference) (OtherActor :type Actor%20Object%20Reference) (OtherComp :type Primitive%20Component%20Object%20Reference) (OtherBodyIndex :type Integer))
  (if (Actor|ActorHasTag OtherActor "Metaphys_1")
    (Variables|Default|SetMetaphys_evil_1 false)
    (Development|PrintString "Hello" :!label _label)
    (elif (Actor|ActorHasTag OtherActor "Metaphys_2")
      (Variables|Default|SetMetaphys_evil_2 false)
      (goto _label)
      (elif (Actor|ActorHasTag OtherActor "Metaphys_3")
        (Variables|Default|SetMetaphys_evil_3 false)
        (goto _label)))))

(event EventNewTryLavka
  (Variables|Default|SetCan_try true)
  (Default|CallRestart))

(event Input|KeyboardEvents|V
  (params (Key :type Key%20Structure :default "None"))
  (bind _returnvalue (Game|GetPlayerController 0))
  (:Pressed
    (bind _returnvalue_2 (UserInterface|CreateWidget "/Game/Quests/quest_3_lavka/Book/Lavka_controls_widget.Lavka_controls_widget_C"))
    (UserInterface|Viewport|AddtoViewport _returnvalue_2 0)
    (Input|SetInputModeUIOnly _returnvalue _returnvalue_2 "DoNotLock")
    (Variables|/Script/Engine.PlayerController|SetbShowMouseCursor _returnvalue true)))

(event Input|KeyboardEvents|C
  (params (Key :type Key%20Structure :default "None"))
  (:Pressed
    (bind _asbp_playable_character (Utilities|Casting|CastToBP_PlayableCharacter (Game|GetPlayerCharacter 0)))
    (if (Variables|/Game/Entities/BP_PlayableCharacter.BP_PlayableCharacter_C|GetisHoldingObject _asbp_playable_character)
      (Default|Drop _asbp_playable_character))
    (if (Variables|Default|GetPhys_evil_1)
      (if (Variables|Default|GetMoral_evil_1)
        (if (Variables|Default|GetMetaphys_evil_1)
          (if (Variables|Default|GetMoral_evil_2)
            (if (Variables|Default|GetPhys_evil_2)
              (if (Variables|Default|GetMetaphys_evil_2)
                (if (Variables|Default|GetMetaphys_evil_3)
                  (if (Variables|Default|GetPhys_evil_3)
                    (if (Variables|Default|GetMoral_evil_3)
                      (Development|PrintString "V I C T O R Y")
                      (Collision|SetCollisionEnabled (Variables|Default|GetInv_wall_1) "NoCollision")
                      (Class|SwitchCameraMode3rd|SwitchCameraMode3rd(Message) (Game|GetPlayerCharacter 0))
                      (Input|DisableInput (Game|GetPlayerController 0))
                      (else
                        (CallFunction|RestartFunc)))
                    (else
                      (CallFunction|RestartFunc)))
                  (else
                    (CallFunction|RestartFunc)))
                (else
                  (CallFunction|RestartFunc)))
              (else
                (CallFunction|RestartFunc)))
            (else
              (CallFunction|RestartFunc)))
          (else
            (CallFunction|RestartFunc)))
        (else
          (CallFunction|RestartFunc)))
      (else
        (CallFunction|RestartFunc)))))

(fn ConstructionScript)

(fn RestartFunc
  (bind _returnvalue (Game|GetPlayerController 0))
  (bind _returnvalue_2 (Game|GetPlayerController 0))
  (Variables|Default|SetCan_try false)
  (Variables|Default|SetNumOfWrongAnswer (+ (Variables|Default|GetNumOfWrongAnswer) 1))
  (bind _asmy_gi (Utilities|Casting|CastToMyGI (Game|GetGameInstance)))
  (Variables|/Game/Quests/Quest_4_Prolet/MyGI.MyGI_C|SetmustGoToBook_3_quest_lavka _asmy_gi true)
  (Collision|SetCollisionEnabled (Variables|Default|GetInv_wall_1) "NoCollision")
  (Class|SwitchCameraMode3rd|SwitchCameraMode3rd(Message) (Game|GetPlayerCharacter 0))
  (Input|DisableInput (Game|GetPlayerController 0))
  (if (== (Variables|Default|GetNumOfWrongAnswer) 1)
    (bind _returnvalue_3 (UserInterface|CreateWidget "/Game/Quests/quest_3_lavka/Bad_first_answer_widget_lavka.Bad_first_answer_widget_lavka_C"))
    (UserInterface|Viewport|AddtoViewport _returnvalue_3 0)
    (Input|SetInputModeUIOnly _returnvalue_2 _returnvalue_3 "DoNotLock")
    (Variables|/Script/Engine.PlayerController|SetbShowMouseCursor _returnvalue_2 true)
    (elif (== (Variables|Default|GetNumOfWrongAnswer) 2)
      (bind _returnvalue_4 (UserInterface|CreateWidget "/Game/Quests/quest_3_lavka/Bad_second_answer_widget_lavka.Bad_second_answer_widget_lavka_C"))
      (UserInterface|Viewport|AddtoViewport _returnvalue_4 0)
      (Input|SetInputModeUIOnly _returnvalue _returnvalue_4 "DoNotLock")
      (Variables|/Script/Engine.PlayerController|SetbShowMouseCursor _returnvalue true)
      (else
        (bind _returnvalue_5 (UserInterface|CreateWidget "/Game/Quests/quest_2_bridge/Matching_end.Matching_end_C"))
        (UserInterface|Viewport|AddtoViewport _returnvalue_5 0))))
  (return))