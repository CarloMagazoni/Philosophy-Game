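; Temple hatch Blueprint that slides a hatch open when anything begins overlapping its Box trigger.
; BeginPlay stores the world location of the Hatch's owning actor as the start position.
; The overlap plays the Hatch_Open timeline, which adds its HatchMovement track to that start and applies it as the owner's relative location with sweep.
; It has no overlap filter or closing logic.
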(event OnComponentBeginOverlap(Box)
  (params (OverlappedComponent :type Primitive%20Component%20Object%20Reference) (OtherActor :type Actor%20Object%20Reference) (OtherComp :type Primitive%20Component%20Object%20Reference) (OtherBodyIndex :type Integer) (bFromSweep :type Boolean) (SweepResult :type Hit%20Result%20Structure%20%28by%20ref%29))
  (bind _hatch_movement (Timeline|Hatch_Open Play)
    (:Update
      (Transformation|SetActorRelativeLocation (Components|GetOwner (Variables|Default|Gethatch)) (+ _hatch_movement (Variables|Default|GetHatch_StartLocation)) true))))

(event EventBeginPlay
  (Variables|Default|SetHatch_StartLocation (Transformation|GetActorLocation (Components|GetOwner (Variables|Default|Gethatch)))))

(fn ConstructionScript)