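; Fog effect actor that builds a fog volume from nested instances of one static mesh.
; The construction script adds instances at the local origin to an InstancedStaticMesh, each scaled uniformly by its index times SpawnScale, with NumberOfInst setting the count.
; DestroyFog removes the actor immediately; a Destroy timeline that would rescale the root is never triggered.
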(event EventDestroyFog
  (Actor|DestroyActor))

(fn ConstructionScript
  (for _index (range 0 (Variables|Default|GetNumberOfInst))
    (Components|InstancedStaticMesh|AddInstance (Variables|Default|GetInstancedStaticMesh) (Math|Transform|MakeTransform "0, 0, 0" "0, 0, 0" (Math|Vector|MakeVector (* _index (Variables|Default|GetSpawnScale)) (* _index (Variables|Default|GetSpawnScale)) (* _index (Variables|Default|GetSpawnScale)))))))