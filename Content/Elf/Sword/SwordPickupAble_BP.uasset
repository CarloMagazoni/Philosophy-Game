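; Pickup actor that lets the player collect a sword when standing near it.
; A Box overlap with the player pawn sets IsNear, toggles input on the actor, and shows or removes a PickUpSwordWidget prompt.
; Pressing Interact while near flags BP_PlayableCharacter as armed, reveals its SwordMeshOnLeg mesh, removes the prompt and destroys the pickup.
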(event OnComponentBeginOverlap(Box)
  (params (OverlappedComponent :type Primitive%20Component%20Object%20Reference) (OtherActor :type Actor%20Object%20Reference) (OtherComp :type Primitive%20Component%20Object%20Reference) (OtherBodyIndex :type Integer) (bFromSweep :type Boolean) (SweepResult :type Hit%20Result%20Structure%20%28by%20ref%29))
  (if (== OtherActor (Game|Player|GetPlayerPawn 0))
    (Variables|Default|SetIsNear true)
    (Input|EnableInput (Game|GetPlayerController 0))
    (if true
      (bind _returnvalue (UserInterface|CreateWidget "/Game/Elf/Sword/PickUpSwordWidget.PickUpSwordWidget_C"))
      (bind _output_get (Variables|Default|SetSwordWidgetRef _returnvalue))
      (UserInterface|Viewport|AddtoViewport _output_get 0))))

(event OnComponentEndOverlap(Box)
  (params (OverlappedComponent :type Primitive%20Component%20Object%20Reference) (OtherActor :type Actor%20Object%20Reference) (OtherComp :type Primitive%20Component%20Object%20Reference) (OtherBodyIndex :type Integer))
  (if (== OtherActor (Game|Player|GetPlayerPawn 0))
    (Variables|Default|SetIsNear false)
    (Input|DisableInput (Game|GetPlayerController 0))
    (Widget|RemovefromParent (Variables|Default|GetSwordWidgetRef))))

(event Input|ActionEvents|InputActionInteract
  (params (Key :type Key%20Structure :default "None"))
  (:Pressed
    (if (Variables|Default|GetIsNear)
      (bind _asbp_playable_character (Utilities|Casting|CastToBP_PlayableCharacter (Game|Player|GetPlayerPawn 0)))
      (Variables|/Game/Entities/BP_PlayableCharacter.BP_PlayableCharacter_C|SetDoesHaveWeapon _asbp_playable_character true)
      (Rendering|SetVisibility (Variables|/Game/Entities/BP_PlayableCharacter.BP_PlayableCharacter_C|GetSwordMeshOnLeg _asbp_playable_character) true false)
      (Widget|RemovefromParent (Variables|Default|GetSwordWidgetRef))
      (Actor|DestroyActor))))

(fn ConstructionScript)